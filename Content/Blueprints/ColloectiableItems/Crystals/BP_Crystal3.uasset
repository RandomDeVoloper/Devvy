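; Crystal collectible actor, the third crystal by name, that reacts when the BP_Devvy character enters its Box trigger.
; On overlap it sets the mesh of Devvy's Crystal component to SM_crystal_group_01, then creates a WBP_TCrystal3 widget and adds it to the viewport.
; The actor neither destroys itself nor guards against repeat triggers, so each new overlap adds another widget.
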(event `self.Box.OnComponentBeginOverlap`
  (params (OverlappedComponent :type "PrimitiveComponent Object Reference") (OtherActor :type "Actor Object Reference") (OtherComp :type "PrimitiveComponent Object Reference") (OtherBodyIndex :type Integer) (bFromSweep :type Boolean) (SweepResult :type "HitResult Structure (by ref)"))
  (bind _asbp_devvy (cast `/Game/Blueprints/Player/BP_Devvy` OtherActor))
  (`StaticMeshComponent.SetStaticMesh` (`/Game/Blueprints/Player/BP_Devvy.Crystal` _asbp_devvy) "/Game/Crystal_cave/Meshes/Crystal/SM_crystal_group_01.SM_crystal_group_01")
  (bind _returnvalue (`|CreateWidget` "/Game/Widgets/WBP_Crystals/WBP_TCrystal3.WBP_TCrystal3_C"))
  (`UserWidget.AddToViewport` _returnvalue 0))

(fn `UserConstructionScript`
  (`parent.UserConstructionScript`))