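; Master Blueprint for collectable fruit items that spin, float and get picked up by BP_Devvy.
; Tick applies a steady yaw rotation, while the FloatingAnim timeline bobs the actor vertically around the mesh's starting world location, scaled by FloatHeight.
; A Box overlap with BP_Devvy plays a collect sound and destroys the actor after a short delay, with no score or inventory update in this graph.
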(event `self.ReceiveTick`
  (params (DeltaSeconds :type "Float (single-precision)"))
  ; Yükselip alçalma animasyon
  (`self.K2_AddActorLocalRotation` (`KismetMathLibrary.MakeRotator` 0.0 0.0 (* DeltaSeconds 30.0))))

(event `self.ReceiveBeginPlay`
  ; Yükselip alçalma animasyon
  (set `self.StartLocation` (`SceneComponent.K2_GetComponentLocation` (`self.StaticMesh`)))
  (bind (_direction _floatoffset_) (`Timeline|FloatingAnim`)
    (:`Update`
      (`self.K2_SetActorLocation` (+ (`self.StartLocation`) (`KismetMathLibrary.MakeVector` 0.0 0.0 (* _floatoffset_ (`self.FloatHeight`))))))))

(event `self.Box.OnComponentBeginOverlap`
  (params (OverlappedComponent :type "PrimitiveComponent Object Reference") (OtherActor :type "Actor Object Reference") (OtherComp :type "PrimitiveComponent Object Reference") (OtherBodyIndex :type Integer) (bFromSweep :type Boolean) (SweepResult :type "HitResult Structure (by ref)"))
  ; Toplama sesi
  (cast `/Game/Blueprints/Player/BP_Devvy` OtherActor)
  (`GameplayStatics.PlaySoundAtLocation` "/Game/Assets/Sounds/SW_Collect1.SW_Collect1" (0.0 0.0 0.0) (struct) 0.2 1.0 0.0 null null null null)
  (`KismetSystemLibrary.Delay` 0.2)
  (`self.K2_DestroyActor`))

(fn `UserConstructionScript`)