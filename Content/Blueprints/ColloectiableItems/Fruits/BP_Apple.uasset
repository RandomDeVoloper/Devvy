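; BP_Apple is an apple collectible that registers a pickup when BP_Devvy overlaps its Box component.
; The overlap sets IsApple on BP_Devvy, increments its HowMuchApple counter, prints the count and adds a new WBP_TApple widget to the viewport.
; Two DoOnce gates wrap this chain but reset right after the widget is added, and the apple is never destroyed in this graph.
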(event `self.Box.OnComponentBeginOverlap`
  (params (OverlappedComponent :type "PrimitiveComponent Object Reference") (OtherActor :type "Actor Object Reference") (OtherComp :type "PrimitiveComponent Object Reference") (OtherBodyIndex :type Integer) (bFromSweep :type Boolean) (SweepResult :type "HitResult Structure (by ref)"))
  (`/Engine/EditorBlueprintResources/StandardMacros.DoOnce` false :!label _label
    (:`Completed`
      (bind _asbp_devvy (cast `/Game/Blueprints/Player/BP_Devvy` OtherActor))
      (set `/Game/Blueprints/Player/BP_Devvy.bIsApple` true _asbp_devvy)
      (bind _result (`/Engine/EditorBlueprintResources/StandardMacros.IncrementFloat` (`/Game/Blueprints/Player/BP_Devvy.HowMuchApple` _asbp_devvy))
        (:`  `
          (`KismetSystemLibrary.PrintString` (`KismetStringLibrary.Concat_StrStr` "Elma adedi:  " (`KismetStringLibrary.Conv_DoubleToString` _result)))
          (`/Engine/EditorBlueprintResources/StandardMacros.DoOnce` false :!label _label_2
            (:`Completed`
              (bind _returnvalue (`|CreateWidget` "/Game/Blueprints/ColloectiableItems/WBP/WBP_TApple.WBP_TApple_C"))
              (`UserWidget.AddToViewport` _returnvalue 0)
              (`|ExecutionSequence`
                (:`then_0`
                  (goto _label :!via `Reset`))
                (:`then_1`
                  (goto _label_2 :!via `Reset`))))))))))

(fn `UserConstructionScript`
  (`parent.UserConstructionScript`))